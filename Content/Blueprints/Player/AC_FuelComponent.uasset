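; Player actor component that tracks a fuel value and treats it like health, with damage, death and refuel operations.
; All changes go through SetFuel, which clamps to the min/max range; getters expose raw fuel, normalized fuel and a dead check.
; Init sets fuel before assigning new limits, so it clamps against the old range.
; BeginPlay immediately applies a fixed damage amount.
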(event EventBeginPlay
  (CallFunction|Damage 25.0))

(event EventTick
  (params (DeltaSeconds :type Float%20%28single-precision%29)))

(fn SetFuel
  (params (NewFuel :type Float%20%28double-precision%29))
  (bind _output_get (Variables|Default|SetFuel (CallFunction|ClampFuel NewFuel)))
  (return _output_get))

(fn GetFuel
  (return (Variables|Default|GetFuel)))

(fn ClampFuel
  (params (Value :type Float%20%28double-precision%29))
  (return (Math|Float|Clamp(Float) Value (Variables|Default|GetMinFuel) (Variables|Default|GetMaxFuel))))

(fn GetNormalizedFuel
  (return (Math|Float|Clamp(Float) (/ (CallFunction|GetFuel) (Variables|Default|GetMaxFuel)))))

(fn Damage
  (params (DamageAmount :type Float%20%28double-precision%29))
  (if (> DamageAmount 0.0)
    (CallFunction|SetFuel (- (CallFunction|GetFuel) DamageAmount))))

(fn Death
  (CallFunction|Damage (Variables|Default|GetMaxFuel)))

(fn IsDead
  (return (<= (CallFunction|GetFuel) (Variables|Default|GetMinFuel))))

(fn Init
  (params (Fuel :type Float%20%28double-precision%29) (Min%20Fuel :type Float%20%28double-precision%29) (Max%20Fuel :type Float%20%28double-precision%29))
  (CallFunction|SetFuel Fuel)
  (Variables|Default|SetMinFuel Min%20Fuel)
  (Variables|Default|SetMaxFuel Max%20Fuel))

(fn Refuel
  (params (Refuel%20Amount :type Float%20%28double-precision%29))
  (if (> Refuel%20Amount 0.0)
    (CallFunction|SetFuel (+ (CallFunction|GetFuel) Refuel%20Amount))))

(fn FullRefuel
  (CallFunction|Refuel (Variables|Default|GetMaxFuel)))