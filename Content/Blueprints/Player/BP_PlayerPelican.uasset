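; Player-controlled pelican character that moves in the world Y-Z plane from Enhanced Input.
; BeginPlay adds the IMC_Player mapping context to the owning player controller.
; IA_Movement maps its X axis to world right and Y axis to world up, feeding AddMovementInput independently of actor rotation.
; Torque and impulse nodes are left unconnected and never run.
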(event Input|EnhancedActionEvents|EnhancedInputActionIA_Movement
  (params (ActionValue :type Vector%202D%20Structure) (ElapsedSeconds :type Float%20%28double-precision%29) (TriggeredSeconds :type Float%20%28double-precision%29) (InputAction :type Input%20Action%20Object%20Reference :default "/Game/Inputs/IA_Movement.IA_Movement"))
  (:Triggered
    (Pawn|Input|AddMovementInput (+ (* (.x ActionValue) (Math|Vector|GetRightVector (Math|Rotator|MakeRotator 0.0 0.0 0.0))) (* (.y ActionValue) (Math|Vector|GetUpVector (Math|Rotator|MakeRotator 0.0 0.0 0.0)))) 1.0 false)))

(event EventBeginPlay
  (bind _asplayer_controller (Utilities|Casting|CastToPlayerController (Pawn|GetController)))
  (Input|AddMappingContext (PlayerController|LocalPlayerSubsystems|GetEnhancedInputLocalPlayerSubsystem _asplayer_controller) "/Game/Inputs/IMC_Player.IMC_Player" 0 "(bIgnoreAllPressedKeysUntilRelease=True,bForceImmediately=False,bNotifyUserSettings=False)"))

(event Collision|EventActorBeginOverlap
  (params (OtherActor :type Actor%20Object%20Reference)))

(event EventTick
  (params (DeltaSeconds :type Float%20%28single-precision%29)))

(fn ConstructionScript)