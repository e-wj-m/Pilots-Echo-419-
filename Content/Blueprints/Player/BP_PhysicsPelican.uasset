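; Player pelican driven by physics forces on its skeletal mesh, steered with thrust and rotation.
; BeginPlay adds the Enhanced Input mapping context and sets a fixed starting rotation.
; Thrust pushes along the mesh's up vector with X zeroed, and Torque spins it around world X by the input value.
; Both use large hardcoded magnitudes and print debug strings, leaving the ForceStrength variable unused.
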(event Input|EnhancedActionEvents|EnhancedInputActionIA_Thrust
  (params (ActionValue :type Float%20%28double-precision%29) (ElapsedSeconds :type Float%20%28double-precision%29) (TriggeredSeconds :type Float%20%28double-precision%29) (InputAction :type Input%20Action%20Object%20Reference :default "/Game/Inputs/IA_Thrust.IA_Thrust"))
  ;[0.15 0.0273 0 0.5] Vertical Player Movement (Force Physics)
  (Development|PrintString "Thrusting >:)")
  (Physics|AddForce (Variables|Default|GetSkeletalMesh) (* (Math|Vector|GetUpVector (Variables|Default|GetSkeletalMesh)) "0.000000,750000000.000000,750000000.000000") "None" false))

(event Input|EnhancedActionEvents|EnhancedInputActionIA_Torque
  (params (ActionValue :type Float%20%28double-precision%29) (ElapsedSeconds :type Float%20%28double-precision%29) (TriggeredSeconds :type Float%20%28double-precision%29) (InputAction :type Input%20Action%20Object%20Reference :default "/Game/Inputs/IA_Torque.IA_Torque"))
  ;[0.03456 0 0.15 0.5] Rotational Movement (Rotational Torque)
  (Development|PrintString "Twerking >:)")
  (Class|PrimitiveComponent|AddTorqueinDegrees (Variables|Default|GetSkeletalMesh) (Math|Vector|MakeVector (* ActionValue 1e+13) 0.0 0.0) "None" false))

(event EventBeginPlay
  ;[0.15 0 0 0.5] Enhanced Input System Initialization
  (bind _asplayer_controller (Utilities|Casting|CastToPlayerController (Game|GetPlayerController 0)))
  (Input|AddMappingContext (PlayerController|LocalPlayerSubsystems|GetEnhancedInputLocalPlayerSubsystem _asplayer_controller) "/Game/Inputs/IMC_Player.IMC_Player" 0 "(bIgnoreAllPressedKeysUntilRelease=True,bForceImmediately=False,bNotifyUserSettings=False)")
  (Transformation|SetActorRotation "0.000000,90.000000,0.000000"))

(fn ConstructionScript)